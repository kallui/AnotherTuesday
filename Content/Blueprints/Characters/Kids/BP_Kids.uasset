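; BP_Kids is a kid character that starts following a Chad character who enters its aggro range.
; When the AggroRange component begins overlapping a BP_Character of a different faction that is also a BP_Chad, it sets that Chad as the follow target on its AIC_EnemyFollow controller.
; BeginPlay, actor overlap and Tick are disabled stubs, so this overlap is the only logic.
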(event OnComponentBeginOverlap(AggroRange)
  (params (OverlappedComponent :type Primitive%20Component%20Object%20Reference) (OtherActor :type Actor%20Object%20Reference) (OtherComp :type Primitive%20Component%20Object%20Reference) (OtherBodyIndex :type Integer) (bFromSweep :type Boolean) (SweepResult :type Hit%20Result%20Structure%20%28by%20ref%29))
  (bind _asbp_character (Utilities|Casting|CastToBP_Character OtherActor))
  (if (!= (Variables|/Game/Blueprints/Characters/BP_Character.BP_Character_C|GetFaction _asbp_character) (Variables|Default|GetFaction))
    (bind _asbp_chad (Utilities|Casting|CastToBP_Chad _asbp_character))
    (bind _asaic_enemy_follow (Utilities|Casting|CastToAIC_EnemyFollow (AI|GetAIController self)))
    (Default|SetFollowTarget _asaic_enemy_follow _asbp_chad)))

(event EventBeginPlay
  (|CallParentFunction) ; This node is disabled and will not be called.\nDrag off pins to build functionality.
)

(event Collision|EventActorBeginOverlap
  (params (OtherActor :type Actor%20Object%20Reference))
  (|CallParentFunction OtherActor) ; This node is disabled and will not be called.\nDrag off pins to build functionality.
)

(event EventTick
  (params (DeltaSeconds :type Float%20%28single-precision%29))
  (|CallParentFunction DeltaSeconds) ; This node is disabled and will not be called.\nDrag off pins to build functionality.
)

(fn ConstructionScript
  (|CallParentFunction))