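; BP_ExWife is the Ex-Wife boss character, which transforms on first aggro and flags itself as killed when health runs out.
; When a character of another faction enters AggroRange, the first trigger starts a Transform animation override.
; That trigger and later overlaps hand any BP_Chad to AIC_Enemy as the attack target, without waiting for the animation to finish.
; Tick watches CurrentHealth and sets BossKilled once through a DoOnce.
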(event OnComponentBeginOverlap(AggroRange)
  (params (OverlappedComponent :type Primitive%20Component%20Object%20Reference) (OtherActor :type Actor%20Object%20Reference) (OtherComp :type Primitive%20Component%20Object%20Reference) (OtherBodyIndex :type Integer) (bFromSweep :type Boolean) (SweepResult :type Hit%20Result%20Structure%20%28by%20ref%29))
  (bind _asbp_character (Utilities|Casting|CastToBP_Character OtherActor))
  (if (!= (Variables|/Game/Blueprints/Characters/BP_Character.BP_Character_C|GetFaction _asbp_character) (Variables|Default|GetFaction))
    (if (Variables|Default|GetTransformed_0)
      _
      (else
        (Variables|Default|SetTransformed_0 true)
        (Variables|Default|SetTransformed true)
        (|PlayAnimationOverridewithCallbacks (Variables|Default|GetAnimInstance) "/Game/Blueprints/Characters/ExWife/AnimSequences/Transform.Transform" "DefaultSlot" 1.0 0.0
          (:then
            _))))
    (bind _asbp_chad (Utilities|Casting|CastToBP_Chad OtherActor))
    (bind _asaic_enemy (Utilities|Casting|CastToAIC_Enemy (AI|GetAIController self)))
    (Default|SetAttackTarget _asaic_enemy _asbp_chad)))

(event EventBeginPlay
  (|CallParentFunction))

(event Collision|EventActorBeginOverlap
  (params (OtherActor :type Actor%20Object%20Reference))
  (|CallParentFunction OtherActor) ; This node is disabled and will not be called.\nDrag off pins to build functionality.
)

(event EventTick
  (params (DeltaSeconds :type Float%20%28single-precision%29))
  (|CallParentFunction DeltaSeconds)
  (if (<= (Variables|Default|GetCurrentHealth) 0.0)
    (Utilities|FlowControl|DoOnce false
      (:Completed
        (Variables|Default|SetbossKilled true)))))

(fn ConstructionScript
  (|CallParentFunction))