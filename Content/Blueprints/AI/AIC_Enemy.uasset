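; AI controller for enemy characters that runs the enemy behavior tree and feeds combat state into its blackboard.
; On BeginPlay it starts the tree and, as a temporary measure, targets the player's BP_Chad pawn.
; On possession it binds to the character's stun and defeat events, mirroring stun state to the blackboard and clearing the attack target when that character is defeated.
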(event Custom|OnStunnedStateChange
  (params (IsStunned :type Boolean))
  (AI|Components|Blackboard|SetValueasBool (Variables|Default|GetBlackboard) (Variables|Default|GetIsStunnedKey) IsStunned))

(event Custom|HandleIsDefeated
  (CallFunction|SetAttackTarget))

(event EventBeginPlay
  (Class|AIController|UseBlackboard "/Game/Blueprints/AI/BB_Enemy.BB_Enemy")
  (AI|RunBehaviorTree "/Game/Blueprints/AI/BT_Enemy.BT_Enemy")
  ;[1 1 1] Temp
  (bind _asbp_chad (Utilities|Casting|CastToBP_Chad (Game|Player|GetPlayerPawn 0)))
  (CallFunction|SetAttackTarget _asbp_chad))

(event EventPossess
  (params (PossessedPawn :type Pawn%20Object%20Reference))
  (bind _asbp_character (Utilities|Casting|CastToBP_Character PossessedPawn))
  (Variables|Default|SetChar _asbp_character)
  (EventDispatchers|BindEventtoStunStateChange _asbp_character (delegate Custom|OnStunnedStateChange))
  (EventDispatchers|BindEventtoIsDefeatedStateChange (Variables|Default|GetChar) (delegate Custom|HandleIsDefeated)))

(fn ConstructionScript)

(fn SetAttackTarget
  (params (AttackTarget :type BP%20Chad%20Object%20Reference))
  (AI|Components|Blackboard|SetValueasObject (Variables|Default|GetBlackboard) (Variables|Default|GetAttackTargetKey) AttackTarget)
  (Variables|Default|SetAttackTarget AttackTarget))